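; BP_AI_Controller is the AI controller for enemy characters, driving them with the BT_FirstEnemyBehaviourTree behavior tree.
; On BeginPlay it starts the tree, stores player 0's character in the PlayerReference blackboard key and caches its pawn as an EnemyCharacter.
; Each tick it compares distance to the player against AttackRange and sets IsPlayerInRange only when within range, so it never clears the key.
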(event EventBeginPlay
  (AI|RunBehaviorTree "/Game/Characters/Enemies/Enemy_Imp/Blueprints/BT_FirstEnemyBehaviourTree.BT_FirstEnemyBehaviourTree")
  (AI|Components|Blackboard|SetValueasObject (Variables|Default|GetBlackboard) (Utilities|Name|MakeLiteralName "PlayerReference") (Game|GetPlayerCharacter 0))
  (bind _asenemy_character (Utilities|Casting|CastToEnemyCharacter (Pawn|GetControlledPawn)))
  (Variables|Default|SetMyActor _asenemy_character))

(event EventTick
  (params (DeltaSeconds :type Float%20%28single-precision%29))
  (bind _returnvalue (Game|GetPlayerCharacter 0))
  (bind _myactor (Variables|Default|GetMyActor))
  (bind _returnvalue_2 (Transformation|GetActorLocation _myactor))
  (bind _returnvalue_3 (Transformation|GetActorLocation _returnvalue))
  (bind _attackrange (Variables|/Script/Roguelike.EnemyCharacter|GetAttackRange _myactor))
  (bind _returnvalue_4 (Math|Vector|Distance(Vector) _returnvalue_3 _returnvalue_2))
  (bind _returnvalue_5 (<= _returnvalue_4 _attackrange))
  (if _returnvalue_5
    (CallFunction|HandlePlayerinRange _returnvalue_5)))

(fn ConstructionScript)

(fn HandlePlayerinRange
  (params (PlayerInRange :type Boolean))
  (AI|Components|Blackboard|SetValueasBool (Variables|Default|GetBlackboard) (Utilities|Name|MakeLiteralName "IsPlayerInRange") PlayerInRange))