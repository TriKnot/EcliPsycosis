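; BP_MovingDoor is a door actor that slides from its starting location by a Destination offset when the player enters its trigger box.
; It stores its origin on BeginPlay, then a timeline lerps the actor's location toward the offset with sweep enabled.
; A DoOnce precedes the player cast, so the first overlap by any actor uses up the trigger, and the door has no return movement.
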(event OnComponentBeginOverlap(Box)
  (params (OverlappedComponent :type Primitive%20Component%20Object%20Reference) (OtherActor :type Actor%20Object%20Reference) (OtherComp :type Primitive%20Component%20Object%20Reference) (OtherBodyIndex :type Integer) (bFromSweep :type Boolean) (SweepResult :type Hit%20Result%20Structure%20%28by%20ref%29))
  (bind _origin (Variables|Default|GetOrigin))
  (Utilities|FlowControl|DoOnce false
    (:Completed
      (Utilities|Casting|CastToBP_PlayerCharacter OtherActor)
      (bind _track (Timeline|MovingBetweenPoints PlayFromStart)
        (:Update
          (Transformation|SetActorLocation (Math|Vector|Lerp(Vector) _origin (+ _origin (Variables|Default|GetDestination)) _track) true false))))))

(event EventBeginPlay
  (Variables|Default|SetOrigin (Transformation|GetActorLocation)))

(event Collision|EventActorBeginOverlap
  (params (OtherActor :type Actor%20Object%20Reference)))

(event EventTick
  (params (DeltaSeconds :type Float%20%28single-precision%29)))

(fn ConstructionScript)