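; Player character Blueprint that links melee combat, dashing and damage feedback to its animation Blueprint and HUD.
; MeleeComponent attacks set animation flags and spawn slash particles, while animation callbacks start, stop and clear attacks.
; HurtBox damage spawns damage text and briefly swaps mesh materials to a flash material.
; BeginPlay also creates phase and health widgets; Tick feeds speed to animation, zeroed while dashing.
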(event OnLightAttack(MeleeComponent)
  (Variables|/Game/Characters/Player/Art/Animations/AnimBP_BastardV1.AnimBP_BastardV1_C|SetLightAttack (Variables|Default|GetAs%20Anim%20BP%20Bastard) true))

(event OnHeavyAttack(MeleeComponent)
  (Variables|/Game/Characters/Player/Art/Animations/AnimBP_BastardV1.AnimBP_BastardV1_C|SetHeavyAttack (Variables|Default|GetAs%20Anim%20BP%20Bastard) true))

(event OnWeaponAbility(MeleeComponent)
  (Variables|/Game/Characters/Player/Art/Animations/AnimBP_BastardV1.AnimBP_BastardV1_C|SetWeaponAbility (Variables|Default|GetAs%20Anim%20BP%20Bastard) true))

(event Custom|AttackStateChanged
  (params (NewAttackState :type Boolean))
  (bind _meleecomponent (Variables|Default|GetMeleeComponent))
  (if NewAttackState
    (Class|Weapon|StartAttack _meleecomponent)
    (else
      (Class|Weapon|StopAttack _meleecomponent))))

(event Custom|OnAttackCompleted
  (Class|Weapon|ClearAttack (Variables|Default|GetMeleeComponent)))

(event Custom|ChangeDashState
  (params (bDashState :type Boolean))
  (Variables|/Game/Characters/Player/Art/Animations/AnimBP_BastardV1.AnimBP_BastardV1_C|SetbDash (Variables|Default|GetAs%20Anim%20BP%20Bastard) bDashState))

(event Custom|OnDashCompleted
  (Variables|Default|SetbCanDoAction true)
  (Variables|Default|SetbCanMove true))

(event Custom|SpawnDamageUI
  (params (DamageAmount :type Float%20%28single-precision%29) (_EffectType :type Attack%20Effect%20Structure))
  (bind _returnvalue (UserInterface|CreateWidget "/Game/UI/DamageUI/WBP_DamageText.WBP_DamageText_C" 0 (Transformation|GetActorLocation) "(R=1.000000,G=0.000000,B=0.104989,A=1.000000)"))
  (Variables|/Game/UI/DamageUI/WBP_DamageText.WBP_DamageText_C|SetDamageToDisplay _returnvalue DamageAmount)
  (UserInterface|Viewport|AddtoViewport _returnvalue 0))

(event Custom|SpawnLightAttackVFX
  (bind _returnvalue (Niagara|SpawnSystemAttached "/Game/Art/VFX/NiagaraSystems/PS_SlashParticle.PS_SlashParticle" (Variables|Default|GetWeaponAbilityBoxPos) "None" "0, 0, 0" "0.000000,90.000000,180.000000" "KeepRelativeOffset" false))
  (Transformation|SetRelativeScale3D _returnvalue "0.220000,0.220000,0.220000"))

(event Custom|SpawnHeavyAttackVFX
  (bind _returnvalue (Niagara|SpawnSystemAttached "/Game/Art/VFX/NiagaraSystems/PS_SlashParticle1.PS_SlashParticle1" (Variables|Default|GetWeaponAbilityBoxPos) "None" "0,40.000000, 0" "-30.000000,90.000000,90.000000" "KeepRelativeOffset" false))
  (Transformation|SetRelativeScale3D _returnvalue "0.350000,0.350000,0.350000"))

(event Custom|FlashDamage
  (params (DamageAmount :type Float%20%28single-precision%29) (_EffectType :type Attack%20Effect%20Structure))
  (for (_ _array_index) (Variables|Default|GetCurrentMaterials)
    (Rendering|Material|SetMaterial (Variables|Character|GetMesh) _array_index (Variables|Default|GetDamageFlash)))
  (Utilities|FlowControl|Delay 0.5)
  (for (_ _array_index_2) (Rendering|Material|GetMaterials (Variables|Character|GetMesh))
    (Rendering|Material|SetMaterial (Variables|Character|GetMesh) _array_index_2 (Utilities|Array|Get(acopy) (Variables|Default|GetCurrentMaterials) _array_index_2))))

(event Custom|SpawnWeaponAbilityVFX
  (bind _returnvalue (Niagara|SpawnSystemAttached "/Game/Art/VFX/NiagaraSystems/PS_SlashWeaponAbility.PS_SlashWeaponAbility" (Variables|Default|GetWeaponAbilityBoxPos) "None" "0.000000,0.000000,-100.000000" "0, 0, 0" "KeepRelativeOffset" false))
  (Transformation|SetRelativeScale3D _returnvalue "0.350000,0.350000,0.350000"))

(event EventBeginPlay
  (bind _asanim_bp_bastard_v1 (Utilities|Casting|CastToAnimBP_BastardV1 (Components|SkeletalMesh|GetAnimInstance (Variables|Character|GetMesh))))
  (bind _output_get (Variables|Default|SetAs%20Anim%20BP%20Bastard _asanim_bp_bastard_v1))
  (EventDispatchers|BindEventtoOnAttackStateChanged _output_get (delegate Custom|AttackStateChanged))
  (EventDispatchers|BindEventtoOnDashStateChanged (delegate Custom|ChangeDashState))
  (EventDispatchers|AssignOnAttackCompleted _output_get (delegate Custom|OnAttackCompleted))
  (EventDispatchers|BindEventtoOnDashCompleted _output_get (delegate Custom|OnDashCompleted))
  (bind _returnvalue (UserInterface|CreateWidget "/Game/UI/PhasesUI/WBP_PhaseUI.WBP_PhaseUI_C"))
  (UserInterface|Viewport|AddtoViewport _returnvalue 0)
  (bind _returnvalue_2 (UserInterface|CreateWidget "/Game/UI/PlayerHealthUI/WBP_HealthBar.WBP_HealthBar_C"))
  (UserInterface|Viewport|AddtoViewport _returnvalue_2 0)
  (EventDispatchers|BindEventtoOnReceivedDamage (Variables|Default|GetHurtBox) (delegate Custom|SpawnDamageUI))
  (bind _asbp_custom_game_instance (Utilities|Casting|CastToBP_CustomGameInstance (Game|GetGameInstance)))
  (Default|SetPlayerCharacterHealth _asbp_custom_game_instance)
  (EventDispatchers|BindEventtoOnLightAttack (Variables|Default|GetMeleeComponent) (delegate Custom|SpawnLightAttackVFX))
  (EventDispatchers|BindEventtoOnHeavyAttack (Variables|Default|GetMeleeComponent) (delegate Custom|SpawnHeavyAttackVFX))
  (EventDispatchers|BindEventtoOnWeaponAbility (Variables|Default|GetMeleeComponent) (delegate Custom|SpawnWeaponAbilityVFX))
  (bind _returnvalue_3 (Rendering|Material|CreateDynamicMaterialInstance "/Game/Art/Characters/SharedMaterials/M_FlashDamage.M_FlashDamage" "None" "None" :!class /Script/Engine.KismetMaterialLibrary))
  (Variables|Default|SetDamageFlash _returnvalue_3)
  (EventDispatchers|BindEventtoOnReceivedDamage (Variables|Default|GetHurtBox) (delegate Custom|FlashDamage))
  (Variables|Default|SetCurrentMaterials (Rendering|Material|GetMaterials (Variables|Character|GetMesh)))
  (bind _returnvalue_4 (Rendering|Material|CreateDynamicMaterialInstance "/Game/Art/Characters/SharedMaterials/M_FlashDamage.M_FlashDamage" "None" "Transient" :!class /Script/Engine.KismetMaterialLibrary)))

(event Collision|EventActorBeginOverlap
  (params (OtherActor :type Actor%20Object%20Reference)))

(event EventTick
  (params (DeltaSeconds :type Float%20%28single-precision%29))
  (bind _as_anim_bp_bastard (Variables|Default|GetAs%20Anim%20BP%20Bastard))
  (Variables|/Game/Characters/Player/Art/Animations/AnimBP_BastardV1.AnimBP_BastardV1_C|SetSpeed _as_anim_bp_bastard (Math|Float|SelectFloat 0.0 (Math|Vector|VectorLength (Variables|/Script/Engine.MovementComponent|GetVelocity (Variables|Character|GetCharacterMovement))) (Variables|/Game/Characters/Player/Art/Animations/AnimBP_BastardV1.AnimBP_BastardV1_C|GetbDash _as_anim_bp_bastard))))

(event EventSetDamageBoxPos
  (params (ParentComp :type Scene%20Component%20Object%20Reference))
  (bind _returnvalue (Transformation|AttachComponentToComponent (Variables|Default|GetWeaponHitBox) ParentComp "None" "SnapToTarget" "SnapToTarget" "SnapToTarget" true))
  (Development|PrintString (Utilities|String|Append "Attaching Hitbox " " : " (Utilities|String|ToString(Boolean) _returnvalue))))

(fn ConstructionScript)