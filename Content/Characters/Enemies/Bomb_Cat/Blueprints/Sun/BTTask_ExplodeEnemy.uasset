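; Behavior tree task that makes an enemy, such as the Bomb Cat, self-destruct in an area explosion.
; It deals AttackDamage through hurt boxes to active enemies within AttackRange, found via the world state subsystem, and to the player if in range.
; It spawns a scaled-up explosion emitter, then kills the pawn by applying its max health as damage.
; The task fails if the controlled pawn is not an EnemyCharacter.
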(event EventReceiveExecuteAI
  (params (OwnerController :type AI%20Controller%20Object%20Reference) (ControlledPawn :type Pawn%20Object%20Reference))
  (bind _attackeffect (Utilities|Struct|MakeAttackEffect))
  (bind _asenemy_character (Utilities|Casting|CastToEnemyCharacter ControlledPawn)
    (:then
      (Variables|Default|SetAs%20Enemy%20Character _asenemy_character)
      (bind _arrayelement (Utilities|Array|ReverseforEachLoop (Class|WorldStateSubSystem|GetActiveEnemiesWithingDistancefromPoint (Subsystems|GetWorldStateSubSystem) (Transformation|GetActorLocation (Variables|Default|GetAs%20Enemy%20Character)) (Variables|/Script/Roguelike.EnemyCharacter|GetAttackRange (Variables|Default|GetAs%20Enemy%20Character))))
        (:LoopBody
          (Class|DamageSystem|TransferDamage (Variables|/Script/Roguelike.EnemyCharacter|GetHurtBox _arrayelement) (Math|Conversions|ToFloat(Integer) (Variables|/Script/Roguelike.EnemyCharacter|GetAttackDamage (Variables|Default|GetAs%20Enemy%20Character))) _attackeffect))
        (:Completed
          (if (<= (Math|Vector|Distance(Vector) (Transformation|GetActorLocation (Class|EnemyCharacter|GetPlayerCharacter (Variables|Default|GetAs%20Enemy%20Character))) (Transformation|GetActorLocation (Variables|Default|GetAs%20Enemy%20Character))) (Variables|/Script/Roguelike.EnemyCharacter|GetAttackRange (Variables|Default|GetAs%20Enemy%20Character)))
            (Class|DamageSystem|TransferDamage(Message) (Variables|/Script/Roguelike.PlayerCharacter|GetHurtBox (Class|EnemyCharacter|GetPlayerCharacter (Variables|Default|GetAs%20Enemy%20Character))) (Math|Conversions|ToFloat(Integer) (Variables|/Script/Roguelike.EnemyCharacter|GetAttackDamage (Variables|Default|GetAs%20Enemy%20Character))) _attackeffect))
          (Effects|SpawnEmitteratLocation "/Game/StarterContent/Particles/P_Explosion.P_Explosion" (Transformation|GetActorLocation (Variables|Default|GetAs%20Enemy%20Character)) "0, 0, 0" "12.000000,12.000000,12.000000")
          (Class|DamageSystem|TransferDamage (Variables|/Script/Roguelike.EnemyCharacter|GetHurtBox (Variables|Default|GetAs%20Enemy%20Character)) (Variables|/Script/Roguelike.EnemyCharacter|GetMaxHealth (Variables|Default|GetAs%20Enemy%20Character)) (Utilities|Struct|MakeAttackEffect))
          (AI|BehaviorTree|FinishExecute true))))
    (:CastFailed
      (AI|BehaviorTree|FinishExecute false))))