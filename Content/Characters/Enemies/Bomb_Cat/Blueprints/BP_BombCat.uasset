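; Bomb cat enemy character that latches onto the player and signals a coming explosion with blinking and a range indicator.
; Taking damage sets GotHit on the AI Blackboard, plays a sound and starts the death blink.
; Overlapping the player's HurtBox attaches it to a mesh socket, sets bIsAttached and starts the attack blink.
; Timelines drive a dynamic material's emissive and show the AttackRange-scaled indicator; Tick feeds speed to the AnimBP.
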(event Custom|ChangeGotHitBB
  (params (DamageAmount :type Float%20%28single-precision%29) (_EffectType :type Attack%20Effect%20Structure))
  (AI|Components|Blackboard|SetValueasBool (Variables|/Script/AIModule.AIController|GetBlackboard (AI|GetAIController self)) (Utilities|Name|MakeLiteralName "GotHit") true)
  (Audio|PlaySound2D "/Game/Sound/SFX/EnemyHit_Cue.EnemyHit_Cue" 0.5 1.0 0.0 0 0))

(event Custom|OnComponentBeginOverlap_Event_0
  (params (OverlappedComponent :type Primitive%20Component%20Object%20Reference) (OtherActor :type Actor%20Object%20Reference) (OtherComp :type Primitive%20Component%20Object%20Reference) (OtherBodyIndex :type Integer) (bFromSweep :type Boolean) (SweepResult :type Hit%20Result%20Structure%20%28by%20ref%29))
  (bind _returnvalue (Utilities|Name|MakeLiteralName "EnemyAttachSocket"))
  (bind _attackrange (Variables|Default|GetAttackRange))
  (bind _returnvalue_2 (/ _attackrange 5e+01))
  (bind _asplayer_character (Utilities|Casting|CastToPlayerCharacter OtherActor))
  (Utilities|Casting|CastToHurtBox OtherComp)
  (Collision|SetActorEnableCollision false)
  (Transformation|SetActorLocation (Transformation|GetSocketLocation (Variables|/Script/Engine.Character|GetMesh _asplayer_character) _returnvalue) false true)
  (Transformation|AttachComponentToComponent (Variables|/Script/Engine.Character|GetMesh _asplayer_character) _returnvalue "SnapToTarget" "KeepWorld" "KeepWorld" false)
  (AI|Components|Blackboard|SetValueasBool (Variables|/Script/AIModule.AIController|GetBlackboard (AI|GetAIController self)) (Utilities|Name|MakeLiteralName "bIsAttached") true)
  (Rendering|Material|SetMaterial (Variables|Character|GetMesh) 2 (Variables|Default|GetBlinkMaterial))
  (bind _blink (Timeline|BlinkTimeAttack PlayFromStart)
    (:Update
      (Rendering|Material|SetScalarParameterValue (Variables|Default|GetBlinkMaterial) "EmissiveAlpha" _blink :!class /Script/Engine.MaterialInstanceDynamic)
      (Transformation|SetRelativeScale3D (Variables|Default|GetExplosionRangeVisibility) (Math|Vector|MakeVector _returnvalue_2 _returnvalue_2 0.0))
      (Rendering|SetVisibility (Variables|Default|GetExplosionRangeVisibility) true false))))

(event Custom|SpawnDamageUI
  (params (DamageAmount :type Float%20%28single-precision%29) (_EffectType :type Attack%20Effect%20Structure))
  (bind _attackrange (Variables|Default|GetAttackRange))
  (bind _returnvalue (/ _attackrange 5e+01))
  (Rendering|Material|SetMaterial (Variables|Character|GetMesh) 2 (Variables|Default|GetBlinkMaterial))
  (bind _blink (Timeline|BlinkTimeDeath PlayFromStart)
    (:Update
      (Rendering|Material|SetScalarParameterValue (Variables|Default|GetBlinkMaterial) "EmissiveAlpha" _blink :!class /Script/Engine.MaterialInstanceDynamic)
      (Transformation|SetRelativeScale3D (Variables|Default|GetExplosionRangeVisibility) (Math|Vector|MakeVector _returnvalue _returnvalue 0.0))
      (Rendering|SetVisibility (Variables|Default|GetExplosionRangeVisibility) true false))))

(event EventBeginPlay
  (EventDispatchers|BindEventtoOnReceivedDamage (Variables|Default|GetHurtBox) (delegate Custom|ChangeGotHitBB))
  (Collision|AssignOnComponentBeginOverlap (Variables|Default|GetCapsuleComponent) (delegate Custom|OnComponentBeginOverlap_Event_0))
  (EventDispatchers|BindEventtoOnReceivedDamage (Variables|Default|GetHurtBox) (delegate Custom|SpawnDamageUI))
  (Variables|Default|SetCurrentMaterial (Rendering|Material|GetMaterials (Variables|Character|GetMesh)))
  (bind _returnvalue (Rendering|Material|CreateDynamicMaterialInstance "/Game/Characters/Enemies/Bomb_Cat/Art/Materials/Cat.Cat" "None" "None" :!class /Script/Engine.KismetMaterialLibrary))
  (Variables|Default|SetBlinkMaterial _returnvalue)
  (bind _asanim_bp_bomb_cat (Utilities|Casting|CastToAnimBP_BombCat (Components|SkeletalMesh|GetAnimInstance (Variables|Character|GetMesh))))
  (Variables|Default|SetAs%20Anim%20BP%20Bomb%20Cat _asanim_bp_bomb_cat))

(event EventTick
  (params (DeltaSeconds :type Float%20%28single-precision%29))
  (Variables|/Game/Characters/Enemies/Bomb_Cat/Art/Animations/AnimBP_BombCat.AnimBP_BombCat_C|SetSpeed (Variables|Default|GetAs%20Anim%20BP%20Bomb%20Cat) (Math|Vector|VectorLength (Variables|/Script/Engine.MovementComponent|GetVelocity (Variables|Character|GetCharacterMovement)))))

(fn ConstructionScript)