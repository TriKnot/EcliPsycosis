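; Heavy melee enemy character that animates its attacks and reacts visibly and audibly to damage.
; Anim Blueprint attack-state callbacks start and stop the MeleeComponent, whose light attack triggers the attack animation and spawns an effect at the AttackBox.
; HurtBox damage shows damage text, briefly swaps a mesh material to a flash, plays a hit sound and refreshes front and back health bars.
; Tick feeds movement speed to the Anim Blueprint.
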(event OnLightAttack(MeleeComponent)
  (Variables|/Game/Characters/Enemies/ItemHeavy_Enemy/Art/Animations/MetalHermit_AnimBlueprint.MetalHermit_AnimBlueprint_C|SetbAttack (Variables|Default|GetAnimBlueprint) true)
  (Niagara|SpawnSystematLocation "/Game/Art/VFX/NiagaraSystems/PS_HeavyEnemyAttackV2.PS_HeavyEnemyAttackV2" (Transformation|GetWorldLocation (Variables|Default|GetAttackBox))))

(event Custom|ReceivedDamage
  (params (DamageAmount :type Float%20%28single-precision%29) (_EffectType :type Attack%20Effect%20Structure))
  (bind _health (Variables|Default|GetHealth))
  (bind _maxhealth (Variables|Default|GetMaxHealth))
  (bind _aswbp_damage_text_second_try (Utilities|Casting|CastToWBP_DamageTextSecondTry (UserInterface|GetWidget (Variables|Default|GetDamageText))))
  (Default|Init _aswbp_damage_text_second_try (Utilities|Text|ToText(Float) DamageAmount "HalfToEven"))
  (Rendering|Material|SetMaterial (Variables|Character|GetMesh) 2 (Variables|Default|GetBlinkMaterial))
  (Utilities|FlowControl|Delay 0.2)
  (Rendering|Material|SetMaterial (Variables|Character|GetMesh) 2 (Variables|Default|GetMaterialToChange))
  (Audio|PlaySound2D "/Game/Sound/SFX/EnemyHit_Cue.EnemyHit_Cue" 0.5 1.0 0.0 0 0)
  (CallFunction|SetEnemyHealthBarPercentage (Variables|Default|GetHealthBar) _health _maxhealth)
  (CallFunction|SetEnemyHealthBarPercentage (Variables|Default|GetHealthBarBackSide) _health _maxhealth))

(event Custom|AttackStateChange
  (params (bIsAttacking :type Boolean))
  (bind _meleecomponent (Variables|Default|GetMeleeComponent))
  (if bIsAttacking
    (Class|Weapon|StartAttack _meleecomponent)
    (else
      (Class|Weapon|StopAttack _meleecomponent))))

(event EventBeginPlay
  (bind _health (Variables|Default|GetHealth))
  (bind _maxhealth (Variables|Default|GetMaxHealth))
  (bind _asmetal_hermit_anim_blueprint (Utilities|Casting|CastToMetalHermit_AnimBlueprint (Components|SkeletalMesh|GetAnimInstance (Variables|Character|GetMesh))))
  (bind _output_get (Variables|Default|SetAnimBlueprint _asmetal_hermit_anim_blueprint))
  (EventDispatchers|BindEventtoCallAttackStateChanged _output_get (delegate Custom|AttackStateChange))
  (EventDispatchers|BindEventtoOnReceivedDamage (Variables|Default|GetHurtBox) (delegate Custom|ReceivedDamage))
  (Variables|Default|SetMaterialToChange (Rendering|Material|GetMaterial (Variables|Character|GetMesh) 2))
  (bind _returnvalue (Rendering|Material|CreateDynamicMaterialInstance "/Game/Art/Characters/SharedMaterials/M_FlashDamage.M_FlashDamage" "None" "None" :!class /Script/Engine.KismetMaterialLibrary))
  (Variables|Default|SetBlinkMaterial _returnvalue)
  (CallFunction|SetEnemyHealthBarPercentage (Variables|Default|GetHealthBar) _health _maxhealth)
  (CallFunction|SetEnemyHealthBarPercentage (Variables|Default|GetHealthBarBackSide) _health _maxhealth))

(event EventTick
  (params (DeltaSeconds :type Float%20%28single-precision%29))
  (Variables|/Game/Characters/Enemies/ItemHeavy_Enemy/Art/Animations/MetalHermit_AnimBlueprint.MetalHermit_AnimBlueprint_C|SetSpeed (Variables|Default|GetAnimBlueprint) (Math|Vector|VectorLength (Variables|/Script/Engine.MovementComponent|GetVelocity (Variables|Character|GetCharacterMovement)))))

(fn ConstructionScript)