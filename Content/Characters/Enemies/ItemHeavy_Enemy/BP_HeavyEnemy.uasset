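; BP_HeavyEnemy is the heavy melee enemy character, linking its MetalHermit animation blueprint to melee combat and damage feedback.
; Tick feeds movement speed to the anim blueprint, and a light attack from MeleeComponent sets its Attack flag.
; The anim blueprint's attack-state callback starts and stops the melee component's attack.
; HurtBox damage spawns damage text, swaps in a dynamic flash material, then restores the originals and plays a hit sound after a short delay.
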(event OnLightAttack(MeleeComponent)
  (Variables|/Game/Characters/Enemies/ItemHeavy_Enemy/Art/Animations/MetalHermit_AnimBlueprint.MetalHermit_AnimBlueprint_C|SetbAttack (Variables|Default|GetAnimBlueprint) true))

(event Custom|ReceivedDamage
  (params (DamageAmount :type Float%20%28single-precision%29) (_EffectType :type Attack%20Effect%20Structure))
  (CallFunction|SpawnDamageText DamageAmount self)
  (CallFunction|ApplyBlinkingMaterial (Variables|Default|GetCurrentMaterials) (Variables|Character|GetMesh) (Variables|Default|GetBlinkMaterial))
  (Utilities|FlowControl|Delay 0.5)
  (CallFunction|RevertMaterial (Variables|Character|GetMesh) (Variables|Default|GetCurrentMaterials))
  (Audio|PlaySound2D "/Game/Sound/SFX/EnemyHit_Cue.EnemyHit_Cue" 0.5 1.0 0.0 0 0))

(event Custom|AttackStateChange
  (params (bIsAttacking :type Boolean))
  (bind _meleecomponent (Variables|Default|GetMeleeComponent))
  (if bIsAttacking
    (Class|Weapon|StartAttack _meleecomponent)
    (else
      (Class|Weapon|StopAttack _meleecomponent))))

(event EventBeginPlay
  (bind _asmetal_hermit_anim_blueprint (Utilities|Casting|CastToMetalHermit_AnimBlueprint (Components|SkeletalMesh|GetAnimInstance (Variables|Character|GetMesh))))
  (bind _output_get (Variables|Default|SetAnimBlueprint _asmetal_hermit_anim_blueprint))
  (EventDispatchers|BindEventtoCallAttackStateChanged _output_get (delegate Custom|AttackStateChange))
  (EventDispatchers|BindEventtoOnReceivedDamage (Variables|Default|GetHurtBox) (delegate Custom|ReceivedDamage))
  (Variables|Default|SetCurrentMaterials (Rendering|Material|GetMaterials (Variables|Character|GetMesh)))
  (bind _returnvalue (Rendering|Material|CreateDynamicMaterialInstance "/Game/Art/Characters/SharedMaterials/M_FlashDamage.M_FlashDamage" "None" "None" :!class /Script/Engine.KismetMaterialLibrary))
  (Variables|Default|SetBlinkMaterial _returnvalue))

(event EventTick
  (params (DeltaSeconds :type Float%20%28single-precision%29))
  (Variables|/Game/Characters/Enemies/ItemHeavy_Enemy/Art/Animations/MetalHermit_AnimBlueprint.MetalHermit_AnimBlueprint_C|SetSpeed (Variables|Default|GetAnimBlueprint) (Math|Vector|VectorLength (Variables|/Script/Engine.MovementComponent|GetVelocity (Variables|Character|GetCharacterMovement)))))

(fn ConstructionScript)