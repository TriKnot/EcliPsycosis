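; BP_TrashImp is a melee enemy character that drives its animation, attacks and damage feedback.
; It feeds movement speed and light-attack requests to AnimBP_Imp, whose attack-state and completion events start, stop and clear the melee component's attack.
; HurtBox damage spawns floating damage text, plays a hit sound, briefly swaps a mesh material to a flash instance and refreshes both health bars.
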(event OnLightAttack(MeleeComponent)
  (Variables|/Game/Characters/Enemies/Enemy_Imp/Art/Animation/AnimBP_Imp.AnimBP_Imp_C|SetbAttack (Variables|Default|GetAs%20Anim%20BP%20Imp) true))

(event Custom|AttackStateChanged
  (params (bIsAttacking :type Boolean))
  (bind _meleecomponent (Variables|Default|GetMeleeComponent))
  (if bIsAttacking
    (Class|Weapon|StartAttack _meleecomponent)
    (Audio|PlaySound2D "/Game/Sound/SFX/ImpAttack_Cue.ImpAttack_Cue" 0.4 1.0 0.0 0 0)
    (else
      (Class|Weapon|StopAttack _meleecomponent))))

(event Custom|OnAttackCompleted
  (Class|Weapon|ClearAttack (Variables|Default|GetMeleeComponent)))

(event Custom|SpawnDamageUI
  (params (DamageAmount :type Float%20%28single-precision%29) (_EffectType :type Attack%20Effect%20Structure))
  (bind _health (Variables|Default|GetHealth))
  (bind _maxhealth (Variables|Default|GetMaxHealth))
  (bind _returnvalue (UserInterface|CreateWidget "/Game/UI/DamageUI/WBP_DamageText.WBP_DamageText_C" 0 (Transformation|GetActorLocation)))
  (Variables|/Game/UI/DamageUI/WBP_DamageText.WBP_DamageText_C|SetDamageToDisplay _returnvalue DamageAmount)
  (UserInterface|Viewport|AddtoViewport _returnvalue 0)
  (Rendering|Material|SetMaterial (Variables|Character|GetMesh) 2 (Variables|Default|GetBlinkMaterial))
  (Utilities|FlowControl|Delay 0.2)
  (Rendering|Material|SetMaterial (Variables|Character|GetMesh) 2 (Variables|Default|GetMaterialToChange))
  (Audio|PlaySound2D "/Game/Sound/SFX/EnemyHit_Cue.EnemyHit_Cue" 0.5 1.0 0.0 0 0)
  (CallFunction|SetEnemyHealthBarPercentage (Variables|Default|GetHealthBar) _health _maxhealth)
  (CallFunction|SetEnemyHealthBarPercentage (Variables|Default|GetHealthBarBackSide) _health _maxhealth))

(event EventBeginPlay
  (bind _health (Variables|Default|GetHealth))
  (bind _maxhealth (Variables|Default|GetMaxHealth))
  (bind _asanim_bp_imp (Utilities|Casting|CastToAnimBP_Imp (Components|SkeletalMesh|GetAnimInstance (Variables|Character|GetMesh))))
  (bind _output_get (Variables|Default|SetAs%20Anim%20BP%20Imp _asanim_bp_imp))
  (EventDispatchers|BindEventtoAttackStateChanged _output_get (delegate Custom|AttackStateChanged))
  (EventDispatchers|BindEventtoOnAttackCompleted _output_get (delegate Custom|OnAttackCompleted))
  (EventDispatchers|BindEventtoOnReceivedDamage (Variables|Default|GetHurtBox) (delegate Custom|SpawnDamageUI))
  (Variables|Default|SetMaterialToChange (Rendering|Material|GetMaterial (Variables|Character|GetMesh) 2))
  (bind _returnvalue (Rendering|Material|CreateDynamicMaterialInstance "/Game/Art/Characters/SharedMaterials/M_FlashDamage.M_FlashDamage" "None" "None" :!class /Script/Engine.KismetMaterialLibrary))
  (Variables|Default|SetBlinkMaterial _returnvalue)
  (CallFunction|SetEnemyHealthBarPercentage (Variables|Default|GetHealthBar) _health _maxhealth)
  (CallFunction|SetEnemyHealthBarPercentage (Variables|Default|GetHealthBarBackSide) _health _maxhealth))

(event EventTick
  (params (DeltaSeconds :type Float%20%28single-precision%29))
  (Variables|/Game/Characters/Enemies/Enemy_Imp/Art/Animation/AnimBP_Imp.AnimBP_Imp_C|SetSpeed (Variables|Default|GetAs%20Anim%20BP%20Imp) (Math|Vector|VectorLength (Variables|/Script/Engine.MovementComponent|GetVelocity (Variables|Character|GetCharacterMovement)))))

(fn ConstructionScript)