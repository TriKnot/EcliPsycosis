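; Behavior tree task that picks a cover location for an enemy character.
; Asks the RogueLikeAIController for cover points within the pawn's attack range, then selects the one furthest from the player.
; If that point clears a small minimum distance from the player, writes it to the CoverLocation blackboard key and succeeds.
; Fails if the point is too close or either cast fails.
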(event EventReceiveExecuteAI
  (params (OwnerController :type AI%20Controller%20Object%20Reference) (ControlledPawn :type Pawn%20Object%20Reference))
  (bind _asenemy_character (Utilities|Casting|CastToEnemyCharacter ControlledPawn)
    (:then
      (bind _asrogue_like_aicontroller (Utilities|Casting|CastToRogueLikeAIController OwnerController)
        (:then
          (bind _output_get (Variables|Default|SetAs%20Rogue%20Like%20AIController _asrogue_like_aicontroller))
          (bind __locations (Class|RogueLikeAIController|FindCoverLocations _output_get (Variables|/Script/Roguelike.EnemyCharacter|GetAttackRange _asenemy_character) (Variables|Default|GetDistance%20from%20Hit) (Variables|Default|GetDegrees%20Of%20Precision) false))
          (bind _returnvalue (Class|RogueLikeAIController|GetFurthestPointfrom (Variables|Default|GetAs%20Rogue%20Like%20AIController) __locations (Transformation|GetActorLocation (Variables|/Script/Roguelike.RogueLikeAIController|GetPlayerCharacter (Variables|Default|GetAs%20Rogue%20Like%20AIController)))))
          (if (> (Math|Vector|Distance(Vector) _returnvalue (Transformation|GetActorLocation (Variables|/Script/Roguelike.RogueLikeAIController|GetPlayerCharacter (Variables|Default|GetAs%20Rogue%20Like%20AIController)))) 5e+01)
            (AI|Components|Blackboard|SetValueasVector (Variables|/Script/AIModule.AIController|GetBlackboard (Variables|Default|GetAs%20Rogue%20Like%20AIController)) (Utilities|Name|MakeLiteralName "CoverLocation") _returnvalue)
            (AI|BehaviorTree|FinishExecute true)
            (else
              (AI|BehaviorTree|FinishExecute false))))
        (:CastFailed
          (AI|BehaviorTree|FinishExecute false :!label _label))))
    (:CastFailed
      (goto _label))))