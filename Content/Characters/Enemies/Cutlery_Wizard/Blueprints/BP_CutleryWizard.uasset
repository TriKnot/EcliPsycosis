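; Cutlery Wizard enemy Blueprint: a ranged attacker that snaps to face the player every tick.
; Its RangedComponent fires from a set fire point, and its attack and reload events drive flags on AnimBP_Wizard.
; HurtBox damage refreshes the health bar, briefly swaps a mesh material slot to an M_FlashDamage dynamic instance, then restores it and plays a hit sound.
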(event OnLightAttack(RangedComponent)
  (Variables|/Game/Characters/Enemies/Cutlery_Wizard/Art/Animations/AnimBP_Wizard.AnimBP_Wizard_C|SetbAttacking (Variables|Default|GetAs%20Anim%20BP) true))

(event OnReloadStateChanged(RangedComponent)
  (params (bReloadState :type Boolean))
  (Variables|/Game/Characters/Enemies/Cutlery_Wizard/Art/Animations/AnimBP_Wizard.AnimBP_Wizard_C|SetbReloading (Variables|Default|GetAs%20Anim%20BP) bReloadState))

(event OnReceivedDamage(HurtBox)
  (params (DamageAmount :type Float%20%28single-precision%29) (_EffectType :type Attack%20Effect%20Structure))
  (CallFunction|SetEnemyHealthBarPercentage (Variables|Default|GetHealthBar) (Variables|Default|GetHealth) (Variables|Default|GetMaxHealth)))

(event Custom|SpawnDamageUI
  (params (DamageAmount :type Float%20%28single-precision%29) (_EffectType :type Attack%20Effect%20Structure))
  (Rendering|Material|SetMaterial (Variables|Character|GetMesh) 1 (Variables|Default|GetBlinkMaterial))
  (Utilities|FlowControl|Delay 0.2)
  (Rendering|Material|SetMaterial (Variables|Character|GetMesh) 1 (Variables|Default|GetMaterialToChange))
  (Audio|PlaySound2D "/Game/Sound/SFX/EnemyHit_Cue.EnemyHit_Cue" 0.5 1.0 0.0 0 0))

(event EventBeginPlay
  (Class|RangedComponent|SetFirePoint (Variables|Default|GetRangedComponent) (Variables|Default|GetFirePoint))
  (EventDispatchers|BindEventtoOnReceivedDamage (Variables|Default|GetHurtBox) (delegate Custom|SpawnDamageUI))
  (Variables|Default|SetMaterialToChange (Rendering|Material|GetMaterial (Variables|Character|GetMesh) 1))
  (bind _returnvalue (Rendering|Material|CreateDynamicMaterialInstance "/Game/Art/Characters/SharedMaterials/M_FlashDamage.M_FlashDamage" "None" "None" :!class /Script/Engine.KismetMaterialLibrary))
  (Variables|Default|SetBlinkMaterial _returnvalue)
  (bind _asanim_bp_wizard (Utilities|Casting|CastToAnimBP_Wizard (Components|SkeletalMesh|GetAnimInstance (Variables|Character|GetMesh))))
  (Variables|Default|SetAs%20Anim%20BP _asanim_bp_wizard)
  (CallFunction|SetEnemyHealthBarPercentage (Variables|Default|GetHealthBar) (Variables|Default|GetHealth) (Variables|Default|GetMaxHealth)))

(event EventTick
  (params (DeltaSeconds :type Float%20%28single-precision%29))
  (bind _self self)
  (Transformation|SetActorRotation _self (Math|Rotator|FindLookatRotation (Transformation|GetActorLocation _self) (Transformation|GetActorLocation (Variables|Default|GetPlayerCharacter _self))) true))

(fn ConstructionScript)