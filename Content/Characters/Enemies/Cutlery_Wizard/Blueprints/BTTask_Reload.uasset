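; Behavior tree task that reloads the ranged weapon of an EnemyCharacter, stored with the Cutlery Wizard enemy.
; It refills the pawn's RangedComponent to maximum ammunition, then waits for that component's reload time.
; Afterwards it sets the HasAmmo blackboard key, signals that the reload state has ended and finishes successfully.
; It fails if the pawn is not an EnemyCharacter or lacks a valid RangedComponent.
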(event EventReceiveExecuteAI
  (params (OwnerController :type AI%20Controller%20Object%20Reference) (ControlledPawn :type Pawn%20Object%20Reference))
  (bind _asenemy_character (Utilities|Casting|CastToEnemyCharacter ControlledPawn)
    (:then
      (Utilities|IsValid (Variables|/Script/Roguelike.EnemyCharacter|GetRangedComponent _asenemy_character)
        (:Is%20Valid
          (bind _output_get (Variables|Default|SetRanged%20Component (Variables|/Script/Roguelike.EnemyCharacter|GetRangedComponent _asenemy_character)))
          (Class|RangedComponent|Reload _output_get (Variables|/Script/Roguelike.RangedComponent|GetMaxAmmunition _output_get))
          (Utilities|FlowControl|Delay (Variables|/Script/Roguelike.RangedComponent|GetReloadTime (Variables|Default|GetRanged%20Component)))
          (AI|Components|Blackboard|SetValueasBool (AI|GetBlackboard _asenemy_character) (Utilities|Name|MakeLiteralName "HasAmmo") true)
          (Default|CallOnReloadStateChanged (Variables|Default|GetRanged%20Component) false)
          (AI|BehaviorTree|FinishExecute true))
        (:Is%20Not%20Valid
          (AI|BehaviorTree|FinishExecute false :!label _label))))
    (:CastFailed
      (goto _label))))