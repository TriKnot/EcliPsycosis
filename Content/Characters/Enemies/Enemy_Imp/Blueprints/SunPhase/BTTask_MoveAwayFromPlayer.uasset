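; Behavior tree task in the Imp enemy's sun phase that moves the controlled pawn away from the player.
; It asks the RogueLikeAIController for a retreat position and runs AIMoveTo only if that point lies beyond a minimum distance from the AI controller's own location.
; The task succeeds when the move completes and fails when the point is too close or the move fails.
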(event EventReceiveExecuteAI
  (params (OwnerController :type AI%20Controller%20Object%20Reference) (ControlledPawn :type Pawn%20Object%20Reference))
  (bind _returnvalue (AI|GetAIController ControlledPawn))
  (bind _asrogue_like_aicontroller (Utilities|Casting|CastToRogueLikeAIController _returnvalue))
  (bind _returnvalue_2 (Class|RogueLikeAIController|FindPositionAwayfromPlayer _asrogue_like_aicontroller))
  (if (> (Math|Vector|Distance(Vector) _returnvalue_2 (Transformation|GetActorLocation _returnvalue)) 5e+02)
    (AI|AIMoveTo ControlledPawn _returnvalue_2 0 5.0 false
      (:OnSuccess
        (AI|BehaviorTree|FinishExecute true))
      (:OnFail
        (AI|BehaviorTree|FinishExecute false)))
    (else
      (AI|BehaviorTree|FinishExecute false))))