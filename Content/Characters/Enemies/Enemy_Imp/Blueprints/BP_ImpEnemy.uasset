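; BP_ImpEnemy is the Imp enemy character Blueprint, linking its melee combat component to its animation Blueprint.
; On BeginPlay it caches AnimBP_Imp and binds to its attack events, which start, stop and clear attacks on the MeleeComponent.
; The component's light attack event sets the AnimBP's Attack flag, and Tick feeds movement velocity magnitude into its Speed.
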(event OnLightAttack(MeleeComponent)
  (Variables|/Game/Characters/Enemies/Enemy_Imp/Art/Animation/AnimBP_Imp.AnimBP_Imp_C|SetbAttack (Variables|Default|GetAs%20Anim%20BP%20Imp) true))

(event Custom|AttackStateChanged
  (params (bIsAttacking :type Boolean))
  (bind _meleecomponent (Variables|Default|GetMeleeComponent))
  (if bIsAttacking
    (Class|Weapon|StartAttack _meleecomponent)
    (else
      (Class|Weapon|StopAttack _meleecomponent))))

(event Custom|OnAttackCompleted
  (Class|Weapon|ClearAttack (Variables|Default|GetMeleeComponent)))

(event EventBeginPlay
  (bind _asanim_bp_imp (Utilities|Casting|CastToAnimBP_Imp (Components|SkeletalMesh|GetAnimInstance (Variables|Character|GetMesh))))
  (bind _output_get (Variables|Default|SetAs%20Anim%20BP%20Imp _asanim_bp_imp))
  (EventDispatchers|BindEventtoAttackStateChanged _output_get (delegate Custom|AttackStateChanged))
  (EventDispatchers|BindEventtoOnAttackCompleted _output_get (delegate Custom|OnAttackCompleted)))

(event EventTick
  (params (DeltaSeconds :type Float%20%28single-precision%29))
  (Variables|/Game/Characters/Enemies/Enemy_Imp/Art/Animation/AnimBP_Imp.AnimBP_Imp_C|SetSpeed (Variables|Default|GetAs%20Anim%20BP%20Imp) (Math|Vector|VectorLength (Variables|/Script/Engine.MovementComponent|GetVelocity (Variables|Character|GetCharacterMovement)))))

(fn ConstructionScript)