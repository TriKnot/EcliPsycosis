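; Behavior tree task for enemy AI that checks whether player 0 is within the controlled EnemyCharacter's DetectionRangeRadius.
; It measures horizontal distance using absolute X and Y world coordinates with Z zeroed, so positions mirrored across the world axes count as close.
; It writes the result to the PlayerInRangeBBKey blackboard bool and finishes with success when in range, failure otherwise.
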(event EventReceiveExecuteAI
  (params (OwnerController :type AI%20Controller%20Object%20Reference) (ControlledPawn :type Pawn%20Object%20Reference))
  (bind _returnvalue (Game|GetPlayerCharacter 0))
  (bind _returnvalue_2 (Transformation|GetActorLocation ControlledPawn))
  (bind _returnvalue_3 (Transformation|GetActorLocation _returnvalue))
  (bind _asenemy_character (Utilities|Casting|CastToEnemyCharacter ControlledPawn))
  (Class|BTFunctionLibrary|SetBlackboardValueasBool (Variables|Default|GetPlayerInRangeBBKey) (<= (Math|Vector|Distance(Vector) (Math|Vector|MakeVector (Math|Float|Absolute(Float) (.x _returnvalue_2)) (Math|Float|Absolute(Float) (.y _returnvalue_2)) 0.0) (Math|Vector|MakeVector (Math|Float|Absolute(Float) (.x _returnvalue_3)) (Math|Float|Absolute(Float) (.y _returnvalue_3)) 0.0)) (Variables|/Script/Roguelike.EnemyCharacter|GetDetectionRangeRadius _asenemy_character)))
  (if (<= (Math|Vector|Distance(Vector) (Math|Vector|MakeVector (Math|Float|Absolute(Float) (.x _returnvalue_2)) (Math|Float|Absolute(Float) (.y _returnvalue_2)) 0.0) (Math|Vector|MakeVector (Math|Float|Absolute(Float) (.x _returnvalue_3)) (Math|Float|Absolute(Float) (.y _returnvalue_3)) 0.0)) (Variables|/Script/Roguelike.EnemyCharacter|GetDetectionRangeRadius _asenemy_character))
    (AI|BehaviorTree|FinishExecute true)
    (else
      (AI|BehaviorTree|FinishExecute false))))